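; BP_NinjaEnemy is an AI enemy that patrols, detects, chases, searches for and sword-attacks the player, and can be stealth-killed.
; A tick-driven enum state machine picks the behavior, moving between four patrol points or random navmesh points when searching.
; Pawn sensing fills a decaying detection meter on the player's UI before chasing starts.
; Overlap boxes set player stealth and damage flags, and attacks land via a forward line trace.
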(event OnComponentBeginOverlap(Box)
  (params (OverlappedComponent :type Primitive%20Component%20Object%20Reference) (OtherActor :type Actor%20Object%20Reference) (OtherComp :type Primitive%20Component%20Object%20Reference) (OtherBodyIndex :type Integer) (bFromSweep :type Boolean) (SweepResult :type Hit%20Result%20Structure%20%28by%20ref%29))
  ;[1 1 1] Combat system
  (bind _asbp_player (Utilities|Casting|CastToBP_Player OtherActor))
  (if (not (Variables|Default|GetChasingPlayer))
    (Variables|/Game/NinjaAssets/Characters/Player/BP_Player.BP_Player_C|SetIsStealth? _asbp_player true)))

(event OnComponentEndOverlap(Box)
  (params (OverlappedComponent :type Primitive%20Component%20Object%20Reference) (OtherActor :type Actor%20Object%20Reference) (OtherComp :type Primitive%20Component%20Object%20Reference) (OtherBodyIndex :type Integer))
  ;[1 1 1] Combat system
  (bind _asbp_player (Utilities|Casting|CastToBP_Player OtherActor))
  (Variables|/Game/NinjaAssets/Characters/Player/BP_Player.BP_Player_C|SetIsStealth? _asbp_player false))

(event OnSeePawn(VisionEnemy(PawnSensing)
  (params (Pawn :type Pawn%20Object%20Reference))
  ;[1 1 1] Control the Sensing Vision Enemy
  (bind _output_get (Variables|Default|SetPawn Pawn))
  (bind _asbp_player (Utilities|Casting|CastToBP_Player _output_get))
  (bind _output_get_2 (Variables|Default|SetAs%20BP%20Player _asbp_player))
  (Variables|Default|SetPerceptPlayer true)
  (bind _enable (Utilities|MacroSetDelayChasing)
    (:Return
      (if _enable
        (Variables|Default|SetChasingPlayer true)
        (Variables|Default|SetSearchingPlayer false)
        (Variables|Default|SetCurrentEnumState "NewEnumerator0")
        (elif (> (Transformation|GetDistanceTo _output_get_2) (- (Variables|/Script/AIModule.PawnSensingComponent|GetSightRadius (Variables|Default|GetVisionEnemy%28PawnSensing)) 3e+02))
          (Variables|Default|SetPerceptPlayer false))))))

(event OnComponentBeginOverlap(CollisionDamage)
  (params (OverlappedComponent :type Primitive%20Component%20Object%20Reference) (OtherActor :type Actor%20Object%20Reference) (OtherComp :type Primitive%20Component%20Object%20Reference) (OtherBodyIndex :type Integer) (bFromSweep :type Boolean) (SweepResult :type Hit%20Result%20Structure%20%28by%20ref%29))
  (bind _asbp_player (Utilities|Casting|CastToBP_Player OtherActor))
  (Variables|/Game/NinjaAssets/Characters/Player/BP_Player.BP_Player_C|SetWasteding _asbp_player true))

(event OnComponentEndOverlap(CollisionDamage)
  (params (OverlappedComponent :type Primitive%20Component%20Object%20Reference) (OtherActor :type Actor%20Object%20Reference) (OtherComp :type Primitive%20Component%20Object%20Reference) (OtherBodyIndex :type Integer))
  (bind _asbp_player (Utilities|Casting|CastToBP_Player OtherActor))
  (Variables|/Game/NinjaAssets/Characters/Player/BP_Player.BP_Player_C|SetWasteding _asbp_player false))

(event Custom|NotSeePawn2
  ;[1 1 1] Control the Sensing Vision Enemy
  (if (Variables|Default|GetChasingPlayer)
    (Utilities|FlowControl|Delay 0.5)
    (if (> (Transformation|GetDistanceTo self (Game|Player|GetPlayerPawn 0)) (Variables|/Script/AIModule.PawnSensingComponent|GetSightRadius (Variables|Default|GetVisionEnemy%28PawnSensing)))
      (Variables|Default|SetPerceptPlayer false)
      (Variables|Default|SetChasingPlayer false)
      (Variables|Default|SetSearchingPlayer true)
      (Variables|Default|SetStateEnemy 1)
      (Class|AIEnemyInterface|ControlState(Message) (Variables|Character|GetMesh) (Variables|Default|GetStateEnemy))
      (Variables|Default|SetCurrentEnumState "NewEnumerator1"))))

(event Custom|Patrol
  ;[1 1 1] Patrol Control Enemy
  (Utilities|FlowControl|Sequence
    (:then_0
      (Utilities|FlowControl|DoOnce false :!label _label
        (:Completed
          (switch int (Variables|Default|GetCurrentLocationControl)
            (:0
              (Variables|Default|SetCurrentLocation (Variables|Default|GetLocation)))
            (:1
              (Variables|Default|SetCurrentLocation (Variables|Default|GetLocation1)))
            (:2
              (Variables|Default|SetCurrentLocation (Variables|Default|GetLocation2)))
            (:3
              (Variables|Default|SetCurrentLocation (Variables|Default|GetLocation3))))
          (AI|AIMoveTo self (Variables|Default|GetCurrentLocation) 0 0.1 false
            (:OnSuccess
              (if (Math|Vector|Equal(Vector) (Variables|Default|GetCurrentLocation) (Transformation|GetActorLocation) 1e+02)
                (Math|Integer|IncrementInt (Variables|Default|GetCurrentLocationControl)
                  (:%20%20
                    (if (> (Variables|Default|GetCurrentLocationControl) 3)
                      (Variables|Default|SetCurrentLocationControl 0))
                    (Animation|PlayAnimMontage "/Game/NinjaAssets/Characters/Player/Animations/Idle/Idle_Montage.Idle_Montage" 1.0 "None")
                    (Utilities|FlowControl|Delay (Math|Random|RandomFloatinRange 2.0 6.0))
                    (Animation|StopAnimMontage "/Game/NinjaAssets/Characters/Player/Animations/Idle/Idle_Montage.Idle_Montage")
                    (goto _label Reset)))))))))
    (:then_1
      (if (Variables|Default|GetBeingKilled)
        (AI|AIMoveTo self (Transformation|GetActorLocation) 0 5.0 false
          (:OnSuccess
            (Variables|Default|SetCurrentEnumState "NewEnumerator3")))))
    (:then_2
      (if (Variables|Default|GetChasingPlayer)
        (AI|AIMoveTo self (Transformation|GetActorLocation) 0 5.0 false
          (:then
            (Variables|Default|SetCurrentEnumState "NewEnumerator0")))))
    (:then_3
      (if (Variables|Default|GetDead)
        (AI|AIMoveTo self (Transformation|GetActorLocation) 0 5.0 false
          (:OnSuccess
            (Variables|Default|SetCurrentEnumState "NewEnumerator3")))))))

(event Custom|Search
  ;[1 1 1] Searching Player System
  (Utilities|FlowControl|Sequence
    (:then_0
      (Utilities|FlowControl|DoOnce false :!label _label
        (:Completed
          (if (not (Variables|Default|GetChasingPlayer))
            (if (Variables|Default|GetSearchingPlayer)
              (bind _randomlocation (Class|NavigationSystemV1|GetRandomLocationinNavigableRadius (Variables|Default|GetPointPlayer) 2.5e+02 0 0))
              (AI|AIMoveTo self _randomlocation 0 5.0 false
                (:OnSuccess
                  (if (Math|Vector|Equal(Vector) (Transformation|GetActorLocation) _randomlocation 1e+02)
                    (Animation|PlayAnimMontage "/Game/NinjaAssets/Characters/Player/Animations/Idle/Idle_Searching_Montage.Idle_Searching_Montage" 1.0 "None")
                    (Utilities|FlowControl|Delay (Math|Random|RandomFloatinRange 4.0 8.0))
                    (Animation|StopAnimMontage "/Game/NinjaAssets/Characters/Player/Animations/Idle/Idle_Searching_Montage.Idle_Searching_Montage")
                    (goto _label Reset)))))))))
    (:then_1
      (if (Variables|Default|GetChasingPlayer)
        (Variables|Default|SetSearchingPlayer false)
        (Animation|StopAnimMontage "/Game/NinjaAssets/Characters/Player/Animations/Idle/Idle_Searching_Montage.Idle_Searching_Montage")
        (AI|AIMoveTo self (Transformation|GetActorLocation) 0 5.0 false
          (:then
            _)
          (:OnSuccess
            _))
        (Variables|Default|SetCurrentEnumState "NewEnumerator0")))
    (:then_2
      (if (Variables|Default|GetBeingKilled)
        (Variables|Default|SetSearchingPlayer false)
        (Animation|StopAnimMontage "/Game/NinjaAssets/Characters/Player/Animations/Idle/Idle_Searching_Montage.Idle_Searching_Montage")
        (AI|AIMoveTo self (Transformation|GetActorLocation) 0 5.0 false)))))

(event Custom|AttackingPlayer
  (params (Delay :type Float%20%28single-precision%29))
  (bind _returnvalue (Transformation|GetActorLocation))
  (Utilities|FlowControl|Delay (- Delay 1.2))
  (if (Variables|Default|GetAttacking)
    (Variables|Default|SetAttacking false)
    (bind _outhit (Collision|LineTraceForObjects _returnvalue (+ _returnvalue (* (Transformation|GetActorForwardVector) 1.4e+02)) (Utilities|Array|MakeArray "ObjectTypeQuery3") false (Utilities|Array|MakeArray self) "ForDuration" true "(R=1.000000,G=0.000000,B=0.000000,A=1.000000)" "(R=0.000000,G=1.000000,B=0.000000,A=1.000000)" 0.3))
    (if (.bBlockingHit (Collision|BreakHitResult _outhit))
      (bind _output_get (Variables|Default|SetHit%20Actor (.HitActor (Collision|BreakHitResult _outhit))))
      (Class|AIEnemyInterface|DamagetoPlayer(Message) _output_get))
    (Utilities|FlowControl|Delay 0.8)
    (Variables|Default|SetChasingPlayer true)
    (Variables|Default|SetAttacking true)
    (Variables|Default|SetInCombat false)
    (bind _output_get_2 (Variables|Default|SetStateEnemy 2))
    (Class|AIEnemyInterface|ControlState(Message) (Variables|Character|GetMesh) _output_get_2)
    (Variables|Default|SetCurrentEnumState "NewEnumerator0")))

(event EventBeginPlay
  ;[1 1 1] Set Enemy Initial Configurations
  (Variables|Default|SetAIControllerClass "/Game/NinjaAssets/Characters/Enemy/BP_AIEnemy.BP_AIEnemy_C")
  (bind _asbp_player (Utilities|Casting|CastToBP_Player (Game|Player|GetPlayerPawn 0)))
  (Variables|Default|SetAs%20BP%20Player _asbp_player)
  (Variables|Default|SetStateEnemy 0)
  (Class|AIEnemyInterface|ControlState(Message) (Variables|Character|GetMesh) (Variables|Default|GetStateEnemy))
  (Variables|Default|SetCurrentEnumState "NewEnumerator2"))

(event EventNotStealthKilled
  ;[1 1 1] Combat system
  (if (> (Variables|Default|GetLife) 0)
    (bind _returnvalue (Animation|PlayAnimMontage "/Game/NinjaAssets/Characters/Player/Animations/Hit/Hit_To_Body_Montage.Hit_To_Body_Montage" 1.0 "None"))
    (Utilities|FlowControl|Delay (- _returnvalue 1.0))
    (Math|Integer|DecrementInt (Variables|Default|GetLife))
    (else
      (Animation|PlayAnimMontage "/Game/NinjaAssets/Characters/Player/Animations/Death/Standing_Death_Forward_01_Montage.Standing_Death_Forward_01_Montage" 1.0 "None")
      (Variables|Default|SetChasingPlayer false)
      (Variables|/Game/NinjaAssets/Characters/Player/BP_Player.BP_Player_C|SetInCombat (Variables|Default|GetAs%20BP%20Player) false)
      (Variables|Default|SetDead true)
      (Variables|Default|SetCurrentEnumState "NewEnumerator3"))))

(event EventTick
  (params (DeltaSeconds :type Float%20%28single-precision%29))
  ;[1 1 1] Control State Actions Enemy - Event Tick
  (Utilities|FlowControl|Sequence
    (:then_0
      (Utilities|FlowControl|DoOnce false :!label _label
        (:Completed
          (switch Utilities|FlowControl|Switch|SwitchonEnumStateEnemy (Variables|Default|GetCurrentEnumState)
            (:NewEnumerator0
              (CallFunction|ChasingPlayer)
              (goto _label Reset))
            (:NewEnumerator1
              (CallFunction|SearchPlayer)
              (goto _label Reset))
            (:NewEnumerator2
              (CallFunction|GotoPatrol)
              (goto _label Reset))
            (:NewEnumerator3
              (CallFunction|Death))
            (:NewEnumerator4
              (CallFunction|AttackPlayer)
              (goto _label Reset))))))
    (:then_1
      (CallFunction|NotSeePawn2))
    (:then_2
      (if (Variables|Default|GetPerceptPlayer)
        (if (> (Transformation|GetDistanceTo (Variables|Default|GetAs%20BP%20Player)) (- (Variables|/Script/AIModule.PawnSensingComponent|GetSightRadius (Variables|Default|GetVisionEnemy%28PawnSensing)) 3e+02))
          (Variables|Default|SetPerceptPlayer false))
        (else
          (Utilities|MacroResetDelayChasing))))
    (:then_3
      (Utilities|MacroUIVisionPlayer))))

(event EventStealthKilled
  ;[1 1 1] Combat system
  (Variables|Default|SetBeingKilled true)
  (bind _returnvalue (Animation|PlayAnimMontage "/Game/NinjaAssets/Characters/Player/Animations/Assassination/EnemyDeathStrangling_Montage.EnemyDeathStrangling_Montage" 1.5 "None"))
  (Utilities|FlowControl|Delay (- _returnvalue 0.1))
  (Variables|Default|SetDead true))

(fn ConstructionScript)

(fn GotoPatrol
  (if (not (Variables|Default|GetChasingPlayer))
    (if (not (Variables|Default|GetSearchingPlayer))
      (Variables|Default|SetStateEnemy 1)
      (Variables|/Script/Engine.CharacterMovementComponent|SetMaxWalkSpeed (Variables|Character|GetCharacterMovement) 3e+02)
      (Class|AIEnemyInterface|ControlState(Message) (Variables|Character|GetMesh) (Variables|Default|GetStateEnemy))
      (CallFunction|Patrol))))

(fn ChasingPlayer
  (bind _as_bp_player (Variables|Default|GetAs%20BP%20Player))
  (bind _returnvalue (Transformation|GetActorLocation _as_bp_player))
  (if (not (Variables|Default|GetInCombat))
    (if (not (Variables|Default|GetSearchingPlayer))
      (if (Variables|Default|GetChasingPlayer)
        (Variables|/Game/NinjaAssets/Characters/Player/BP_Player.BP_Player_C|SetInCombat (Variables|Default|GetAs%20BP%20Player) true)
        (Variables|/Script/Engine.CharacterMovementComponent|SetMaxWalkSpeed (Variables|Character|GetCharacterMovement) 6e+02)
        (Variables|Default|SetStateEnemy 2)
        (Variables|/Game/NinjaAssets/Characters/Player/BP_Player.BP_Player_C|SetFocusEnemy _as_bp_player self)
        (Class|AIEnemyInterface|ControlState(Message) (Variables|Character|GetMesh) (Variables|Default|GetStateEnemy))
        (AI|Navigation|SimpleMovetoLocation (AI|GetAIController self) (- _returnvalue 2e+01))
        (if (Math|Vector|Equal(Vector) (Transformation|GetActorLocation) _returnvalue 1.5e+02)
          (AI|Navigation|SimpleMovetoLocation (AI|GetAIController self) (Transformation|GetActorLocation))
          (Variables|Default|SetCurrentEnumState "NewEnumerator4")
          (else
            (CallFunction|NotSeePawn2)))))))

(fn SearchPlayer
  (if (not (Variables|Default|GetInCombat))
    (if true
      (if (not (Variables|Default|GetChasingPlayer))
        (if (not (Variables|Default|GetBeingKilled))
          (Variables|/Game/NinjaAssets/Characters/Player/BP_Player.BP_Player_C|SetInCombat (Variables|Default|GetAs%20BP%20Player) false)
          (Variables|/Script/Engine.CharacterMovementComponent|SetMaxWalkSpeed (Variables|Character|GetCharacterMovement) 4.5e+02)
          (CallFunction|Search))))))

(fn Death
  (Components|Activation|Deactivate (Variables|Default|GetVisionEnemy%28PawnSensing))
  (Utilities|IsValid (Variables|Collision|GetCapsuleComponent)
    (:Is%20Valid
      (Components|DestroyComponent (Variables|Default|GetBox)))
    (:Is%20Not%20Valid
      _))
  (Audio|Components|Audio|Stop (Variables|Character|GetMesh)))

(fn AttackPlayer
  (if (not (Variables|Default|GetDead))
    (Variables|Default|SetInCombat true)
    (Variables|Default|SetChasingPlayer false)
    (Variables|Default|SetStateEnemy 0)
    (Class|AIEnemyInterface|ControlState(Message) (Variables|Character|GetMesh) (Variables|Default|GetStateEnemy))
    (Transformation|SetActorRotation (Class|KismetMathLibrary|RInterptoConstant (Transformation|GetActorRotation) (Math|Rotator|FindLookatRotation (Transformation|GetActorLocation) (Transformation|GetActorLocation (Variables|Default|GetAs%20BP%20Player))) (Utilities|Time|GetWorldDeltaSeconds) 0.0))
    (bind _returnvalue (Animation|PlayAnimMontage "/Game/NinjaAssets/Characters/Player/Animations/Combat/Sword/Attack/Stable_Sword_Inward_Slash_Montage.Stable_Sword_Inward_Slash_Montage" 1.5 "None"))
    (CallFunction|AttackingPlayer _returnvalue)))

(fn AttackerLocation
  (return (Transformation|GetWorldTransform (Variables|Default|GetAttackerLocation1))))