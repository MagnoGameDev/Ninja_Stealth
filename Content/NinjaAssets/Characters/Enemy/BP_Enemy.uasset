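; Enemy character for a ninja game that patrols, chases and searches for the player, and can be stealth-killed or fought.
; Tick runs an enum state machine driving AI moves, walk speed and mesh state messages across a four-point patrol, chase and random-point search.
; Pawn sensing starts the chase, and exceeding sight radius switches to searching.
; A box overlap sets the player's stealth flag, while kill events play montages, reduce life or disable collision.
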(event OnComponentBeginOverlap(Box)
  (params (OverlappedComponent :type Primitive%20Component%20Object%20Reference) (OtherActor :type Actor%20Object%20Reference) (OtherComp :type Primitive%20Component%20Object%20Reference) (OtherBodyIndex :type Integer) (bFromSweep :type Boolean) (SweepResult :type Hit%20Result%20Structure%20%28by%20ref%29))
  ;[1 1 1] Combat system
  (bind _asbp_player (Utilities|Casting|CastToBP_Player OtherActor))
  (Variables|/Game/NinjaAssets/Characters/Player/BP_Player.BP_Player_C|SetIsStealth? _asbp_player true))

(event OnComponentEndOverlap(Box)
  (params (OverlappedComponent :type Primitive%20Component%20Object%20Reference) (OtherActor :type Actor%20Object%20Reference) (OtherComp :type Primitive%20Component%20Object%20Reference) (OtherBodyIndex :type Integer))
  ;[1 1 1] Combat system
  (bind _asbp_player (Utilities|Casting|CastToBP_Player OtherActor))
  (Variables|/Game/NinjaAssets/Characters/Player/BP_Player.BP_Player_C|SetIsStealth? _asbp_player false))

(event OnSeePawn(VisionEnemy(PawnSensing)
  (params (Pawn :type Pawn%20Object%20Reference))
  ;[1 1 1] Control the Sensing Vision Enemy
  (bind _output_get (Variables|Default|SetPawn Pawn))
  (bind _asbp_player (Utilities|Casting|CastToBP_Player _output_get))
  (Variables|Default|SetAs%20BP%20Player _asbp_player)
  (Variables|Animation|SetChasingPlayer true)
  (Variables|Animation|SetSearchingPlayer false)
  (Variables|Animation|SetCurrentEnumState "NewEnumerator0"))

(event Custom|NotSeePawn
  ;[1 1 1] Control the Sensing Vision Enemy
  (if (Variables|Animation|GetChasingPlayer)
    (Utilities|FlowControl|Delay 0.5)
    (if (> (Transformation|GetDistanceTo self (Game|Player|GetPlayerPawn 0)) (Variables|/Script/AIModule.PawnSensingComponent|GetSightRadius (Variables|Default|GetVisionEnemy%28PawnSensing)))
      (Variables|Animation|SetChasingPlayer false)
      (Variables|Animation|SetSearchingPlayer true)
      (Variables|Animation|SetStateEnemy 1)
      (Class|AIEnemyInterface|ControlState(Message) (Variables|Character|GetMesh) (Variables|Animation|GetStateEnemy))
      (Variables|Animation|SetCurrentEnumState "NewEnumerator1"))))

(event Custom|Patrol
  ;[1 1 1] Patrol Control Enemy
  (Utilities|FlowControl|Sequence
    (:then_0
      (Utilities|FlowControl|DoOnce false :!label _label
        (:Completed
          (switch int (Variables|IA|GetCurrentLocationControl)
            (:0
              (Variables|IA|SetCurrentLocation (Variables|IA|GetLocation)))
            (:1
              (Variables|IA|SetCurrentLocation (Variables|IA|GetLocation1)))
            (:2
              (Variables|IA|SetCurrentLocation (Variables|IA|GetLocation2)))
            (:3
              (Variables|IA|SetCurrentLocation (Variables|IA|GetLocation3))))
          (AI|AIMoveTo self (Variables|IA|GetCurrentLocation) 0 0.1 false
            (:OnSuccess
              (if (Math|Vector|Equal(Vector) (Variables|IA|GetCurrentLocation) (Transformation|GetActorLocation) 1e+02)
                (Math|Integer|IncrementInt (Variables|IA|GetCurrentLocationControl)
                  (:%20%20
                    (if (> (Variables|IA|GetCurrentLocationControl) 3)
                      (Variables|IA|SetCurrentLocationControl 0))
                    (Animation|PlayAnimMontage "/Game/NinjaAssets/Characters/Player/Animations/Idle/Idle_Montage.Idle_Montage" 1.0 "None")
                    (Utilities|FlowControl|Delay (Math|Random|RandomFloatinRange 2.0 6.0))
                    (Animation|StopAnimMontage "/Game/NinjaAssets/Characters/Player/Animations/Idle/Idle_Montage.Idle_Montage")
                    (goto _label Reset)))))))))
    (:then_1
      (if (Variables|Animation|GetBeingKilled)
        (AI|AIMoveTo self (Transformation|GetActorLocation) 0 5.0 false)))
    (:then_2
      (if (Variables|Animation|GetChasingPlayer)
        (AI|AIMoveTo self (Transformation|GetActorLocation) 0 5.0 false
          (:then
            (Variables|Animation|SetCurrentEnumState "NewEnumerator0")))))))

(event Custom|Search
  ;[1 1 1] Searching Player System
  (Utilities|FlowControl|Sequence
    (:then_0
      (Utilities|FlowControl|DoOnce false :!label _label
        (:Completed
          (if (not (Variables|Animation|GetChasingPlayer))
            (if (Variables|Animation|GetSearchingPlayer)
              (bind _randomlocation (Class|NavigationSystemV1|GetRandomLocationinNavigableRadius (Variables|IA|GetPointPlayer) 2.5e+02 0 0))
              (AI|AIMoveTo self _randomlocation 0 5.0 false
                (:OnSuccess
                  (if (Math|Vector|Equal(Vector) (Transformation|GetActorLocation) _randomlocation 1e+02)
                    (Animation|PlayAnimMontage "/Game/NinjaAssets/Characters/Player/Animations/Idle/Idle_Searching_Montage.Idle_Searching_Montage" 1.0 "None")
                    (Utilities|FlowControl|Delay (Math|Random|RandomFloatinRange 4.0 8.0))
                    (Animation|StopAnimMontage "/Game/NinjaAssets/Characters/Player/Animations/Idle/Idle_Searching_Montage.Idle_Searching_Montage")
                    (goto _label Reset)
                    (else
                      (Development|PrintString "Hello"))))))))))
    (:then_1
      (if (Variables|Animation|GetChasingPlayer)
        (Variables|Animation|SetSearchingPlayer false)
        (Animation|StopAnimMontage "/Game/NinjaAssets/Characters/Player/Animations/Idle/Idle_Searching_Montage.Idle_Searching_Montage")
        (AI|AIMoveTo self (Transformation|GetActorLocation) 0 5.0 false
          (:then
            _)
          (:OnSuccess
            _))
        (Variables|Animation|SetCurrentEnumState "NewEnumerator0")))
    (:then_2
      (if (Variables|Animation|GetBeingKilled)
        (Variables|Animation|SetSearchingPlayer false)
        (Animation|StopAnimMontage "/Game/NinjaAssets/Characters/Player/Animations/Idle/Idle_Searching_Montage.Idle_Searching_Montage")
        (AI|AIMoveTo self (Transformation|GetActorLocation) 0 5.0 false)))))

(event EventBeginPlay
  ;[1 1 1] Set Enemy Initial Configurations
  (Variables|Default|SetAIControllerClass "/Game/NinjaAssets/Characters/Enemy/BP_AIEnemy.BP_AIEnemy_C")
  (Variables|Animation|SetStateEnemy 0)
  (Class|AIEnemyInterface|ControlState(Message) (Variables|Character|GetMesh) (Variables|Animation|GetStateEnemy))
  (Variables|Animation|SetCurrentEnumState "NewEnumerator2"))

(event EventStealthKilled
  ;[1 1 1] Combat system
  (Variables|Animation|SetBeingKilled true)
  (bind _returnvalue (Animation|PlayAnimMontage "/Game/NinjaAssets/Characters/Player/Animations/Assassination/EnemyDeathStrangling_Montage.EnemyDeathStrangling_Montage" 1.5 "None"))
  (Utilities|FlowControl|Delay (- _returnvalue 0.1))
  (Collision|SetCollisionEnabled (Variables|Collision|GetCapsuleComponent) "NoCollision"))

(event EventNotStealthKilled
  ;[1 1 1] Combat system
  (if (> (Variables|Character|GetLife) 0)
    (bind _returnvalue (Animation|PlayAnimMontage "/Game/NinjaAssets/Characters/Player/Animations/Hit/Hit_To_Body_Montage.Hit_To_Body_Montage" 1.0 "None"))
    (Utilities|FlowControl|Delay (- _returnvalue 1.0))
    (Math|Integer|DecrementInt (Variables|Character|GetLife))
    (else
      (Collision|SetCollisionEnabled (Variables|Collision|GetCapsuleComponent) "NoCollision")
      (bind _returnvalue_2 (Animation|PlayAnimMontage "/Game/NinjaAssets/Characters/Player/Animations/Death/Standing_Death_Forward_01_Montage.Standing_Death_Forward_01_Montage" 1.0 "None"))
      (Utilities|FlowControl|Delay (- _returnvalue_2 1.0)))))

(event EventTick
  (params (DeltaSeconds :type Float%20%28single-precision%29))
  ;[1 1 1] Control State Actions Enemy - Event Tick
  (Utilities|FlowControl|Sequence
    (:then_0
      (Utilities|FlowControl|DoOnce false :!label _label
        (:Completed
          (switch Utilities|FlowControl|Switch|SwitchonEnumStateEnemy (Variables|Animation|GetCurrentEnumState)
            (:NewEnumerator0
              (CallFunction|ChasingPlayer)
              (goto _label Reset))
            (:NewEnumerator1
              (CallFunction|SearchPlayer)
              (goto _label Reset))
            (:NewEnumerator2
              (CallFunction|GotoPatrol)
              (goto _label Reset))))))
    (:then_1
      (CallFunction|NotSeePawn))))

(fn ConstructionScript)

(fn GotoPatrol
  (if (not (Variables|Animation|GetChasingPlayer))
    (if (not (Variables|Animation|GetSearchingPlayer))
      (Variables|Animation|SetStateEnemy 1)
      (Variables|/Script/Engine.CharacterMovementComponent|SetMaxWalkSpeed (Variables|Character|GetCharacterMovement) 3e+02)
      (Class|AIEnemyInterface|ControlState(Message) (Variables|Character|GetMesh) (Variables|Animation|GetStateEnemy))
      (CallFunction|Patrol))))

(fn SearchPlayer
  (if (not (Variables|Animation|GetChasingPlayer))
    (if (not (Variables|Animation|GetBeingKilled))
      (Variables|/Script/Engine.CharacterMovementComponent|SetMaxWalkSpeed (Variables|Character|GetCharacterMovement) 4.5e+02)
      (CallFunction|Search))))

(fn ChasingPlayer
  (if (not (Variables|Animation|GetSearchingPlayer))
    (if (Variables|Animation|GetChasingPlayer)
      (Variables|/Script/Engine.CharacterMovementComponent|SetMaxWalkSpeed (Variables|Character|GetCharacterMovement) 6e+02)
      (Variables|Animation|SetStateEnemy 2)
      (Class|AIEnemyInterface|ControlState(Message) (Variables|Character|GetMesh) (Variables|Animation|GetStateEnemy))
      (AI|Navigation|SimpleMovetoActor (AI|GetAIController self) (Game|GetPlayerCharacter 0))
      (CallFunction|NotSeePawn))))

(fn AttackerLocation
  (return (Transformation|GetWorldTransform (Variables|Default|GetAttackerLocation_0))))